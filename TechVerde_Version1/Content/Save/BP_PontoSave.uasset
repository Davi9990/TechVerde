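; BP_PontoSave is a night-only save point that writes a save when the player presses E inside its zone.
; AtualizarEstadoDoPontoSave shows the actor and enables its collision at night, hiding and disabling it otherwise.
; Box overlaps with BP_Fznd toggle this actor's input.
; E checks Cylinder visibility, saves a newly created BP_MeuSave, with no fields populated here, to a fixed slot and prints the result.
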(event `AtualizarEstadoDoPontoSave`
  (params (`EstaDeNoite?` :type Boolean))
  ; Se estiver de noite, o cilindro aparece e tem colisão overlap. Se não, o cilindro não aparece.
  (if `EstaDeNoite?`
    (`self.SetActorHiddenInGame` false)
    (`self.SetActorEnableCollision` true)
    (else
      (`self.SetActorHiddenInGame` true)
      (`self.SetActorEnableCollision` false))))

(event `Key|E`
  (params (Key :type "Key Structure"))
  ; Condição para salvar se pressionar E no cilindro. O cilindro deve estar visível para que isso aconteca. Apertando E, salva o game na pasta Saved Games do projeto.
  (:`Pressed`
    (if (`SceneComponent.IsVisible` (`self.Cylinder`))
      (bind _returnvalue (`GameplayStatics.CreateSaveGameObject` "/Game/Save/BP_MeuSave.BP_MeuSave_C"))
      (bind _returnvalue_2 (`GameplayStatics.SaveGameToSlot` _returnvalue "Save01"))
      (if _returnvalue_2
        (`KismetSystemLibrary.PrintString` "Jogo salvo com sucesso!" true true (struct :`R` 0.068584 :`G` 1.0 :`A` 1.0))
        (else
          (`KismetSystemLibrary.PrintString` "Erro! Jogo nao salvou" true true (struct :`R` 1.0 :`B` 0.028742 :`A` 1.0)))))))

(event `self.Box.OnComponentBeginOverlap`
  (params (OverlappedComponent :type "PrimitiveComponent Object Reference") (OtherActor :type "Actor Object Reference") (OtherComp :type "PrimitiveComponent Object Reference") (OtherBodyIndex :type Integer) (bFromSweep :type Boolean) (SweepResult :type "HitResult Structure (by ref)"))
  ; Detecta se o player entrou na colisão ou não. Isso evita que o jogador possa apertar E fora da zona de save.
  (cast `/Game/BluePrints/Fznd/BP_Fznd` OtherActor)
  (`self.EnableInput` (`GameplayStatics.GetPlayerController` 0)))

(event `self.Box.OnComponentEndOverlap`
  (params (OverlappedComponent :type "PrimitiveComponent Object Reference") (OtherActor :type "Actor Object Reference") (OtherComp :type "PrimitiveComponent Object Reference") (OtherBodyIndex :type Integer))
  ; Detecta se o player entrou na colisão ou não. Isso evita que o jogador possa apertar E fora da zona de save.
  (cast `/Game/BluePrints/Fznd/BP_Fznd` OtherActor)
  (`self.DisableInput` (`GameplayStatics.GetPlayerController` 0)))

(fn `UserConstructionScript`)