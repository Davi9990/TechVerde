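; BP_Porco is a pig animal actor that patrols a looping route of waypoints.
; On BeginPlay it starts FollowWaypoint, which uses AIMoveTo toward the current entry in the Waypoint array.
; On success it advances the index, wraps to zero at the end, waits briefly and calls itself again.
; Only the success result is handled, so a failed move ends the patrol.
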(event `self.ReceiveBeginPlay`
  (`self.Follow Waypoint`))

(event `Follow Waypoint`
  (`|AIMoveTo` self (0.0 0.0 0.0) (`|GetArrayItem` (`self.Waypoint`) (`self.CurrectWay`))
    (:`OnSuccess`
      (`/Engine/EditorBlueprintResources/StandardMacros.IncrementInt` (`self.CurrectWay`)
        (:`  `
          (if (>= (`self.CurrectWay`) (`KismetArrayLibrary.Array_Length` (`self.Waypoint`)))
            (set `self.CurrectWay` 0))
          (`KismetSystemLibrary.Delay` 1.0)
          (`self.Follow Waypoint`))))))

(fn `UserConstructionScript`)