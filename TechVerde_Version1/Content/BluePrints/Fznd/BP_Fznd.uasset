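; BP_Fznd is the player character, with run, jump, axis-driven movement and turning, and seed-planting interaction.
; On BeginPlay it shows a minimap and creates an inventory widget, which E toggles along with cursor and input mode.
; Mouse buttons fire camera line traces that send Activate or PlantSeed messages to the hit actor, while the wheel adjusts a clamped Seed index.
; Tab disables character movement when an overlapping actor implements an interface.
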(event `Key|E`
  (params (Key :type "Key Structure"))
  (bind _returnvalue (`GameplayStatics.GetPlayerController` 0))
  (bind _returnvalue_2 (`GameplayStatics.GetPlayerController` 0))
  (:`Pressed`
    (`/Engine/EditorBlueprintResources/StandardMacros.FlipFlop`
      (:`A`
        (`UserWidget.AddToViewport` (stale `self.ReceiveBeginPlay` _returnvalue_2) 0)
        (`WidgetBlueprintLibrary.SetInputMode_GameAndUIEx` _returnvalue null)
        (set `PlayerController.bShowMouseCursor` true _returnvalue))
      (:`B`
        (`Widget.RemoveFromParent` (stale `self.ReceiveBeginPlay` _returnvalue_2))
        (`WidgetBlueprintLibrary.SetInputMode_GameOnly` _returnvalue_2)
        (set `PlayerController.bShowMouseCursor` false _returnvalue_2)))))

(event `self.ReceiveBeginPlay`
  ; Mini_Map
  (bind _asplayer_controller (cast `PlayerController` (`self.GetController`)))
  (`/Engine/EditorBlueprintResources/StandardMacros.IsValid` (pcsubsystem `EnhancedInputLocalPlayerSubsystem` _asplayer_controller)
    (:`Is Valid`
      (bind _returnvalue (`|CreateWidget` "/Game/MiniMap/MiniMap_Fznd.MiniMap_Fznd_C" (`GameplayStatics.GetPlayerController` 0)))
      (`UserWidget.AddToViewport` _returnvalue 0)
      (bind _returnvalue_2 (`|GenericCreateObject` (`GameplayStatics.GetPlayerController` 0) "/Game/BluePrints/Inventario/Inventario_UI.Inventario_UI_C")))))

(event `InputAction|Fznd_Run`
  (params (Key :type "Key Structure"))
  (bind _charactermovement (`self.CharacterMovement`))
  ; Correr_Runnig
  (:`Pressed`
    (set `CharacterMovementComponent.MaxWalkSpeed` 600.0 _charactermovement))
  (:`Released`
    (set `CharacterMovementComponent.MaxWalkSpeed` 300.0 _charactermovement)))

(event `Key|Tab`
  (params (Key :type "Key Structure"))
  (:`Pressed`
    (for _array_element (`self.GetOverlappingActors` null)
      (if (`KismetSystemLibrary.DoesImplementInterface` _array_element)
        (`ActorComponent.SetActive` (`self.CharacterMovement`) false false)))))

(event `InputAxis|Fznd_MoveForward`
  (params (AxisValue :type "Float (single-precision)"))
  ; Move_Moviment
  (`self.AddMovementInput` (`SceneComponent.GetRightVector` (`self.CapsuleComponent`)) AxisValue))

(event `InputAxis|Fznd_MoveRight`
  (params (AxisValue :type "Float (single-precision)"))
  ; Move_Moviment
  (`self.AddMovementInput` (`SceneComponent.GetForwardVector` (`self.CapsuleComponent`)) AxisValue))

(event `InputAxis|Fznd_Turn`
  (params (AxisValue :type "Float (single-precision)"))
  ; Turn_Virar
  (`self.AddControllerYawInput` AxisValue))

(event `InputAction|Fznd_Jump`
  (params (Key :type "Key Structure"))
  ; Pula_Jump
  (:`Pressed`
    (`self.Jump`)))

(event `Key|RightMouseButton`
  (params (Key :type "Key Structure"))
  (bind _camera (`self.Camera`))
  (bind _returnvalue (`SceneComponent.K2_GetComponentLocation` _camera))
  (:`Pressed`
    (bind _outhit (`KismetSystemLibrary.LineTraceSingle` :`Start` _returnvalue :`End` (+ _returnvalue (* (`KismetMathLibrary.GetForwardVector` (`SceneComponent.K2_GetComponentRotation` _camera)) 2000.0)) :`TraceChannel` "TraceTypeQuery1" :`DrawDebugType` "ForDuration"))
    (message `/Game/BluePrints/Plants/Plantation/BPI_Activate.Activate` (`.HitActor` (`GameplayStatics.BreakHitResult` _outhit)))))

(event `Key|LeftMouseButton`
  (params (Key :type "Key Structure"))
  (bind _camera (`self.Camera`))
  (bind _returnvalue (`SceneComponent.K2_GetComponentLocation` _camera))
  (:`Pressed`
    (bind _outhit (`KismetSystemLibrary.LineTraceSingle` :`Start` _returnvalue :`End` (+ _returnvalue (* (`KismetMathLibrary.GetForwardVector` (`SceneComponent.K2_GetComponentRotation` _camera)) 2000.0)) :`TraceChannel` "TraceTypeQuery1" :`DrawDebugType` "ForDuration"))
    (message `/Game/BluePrints/Plants/Plantation/BPI_PlantSeed.PlantSeed` (`.HitActor` (`GameplayStatics.BreakHitResult` _outhit)))))

(event `Key|MouseScrollUp`
  (params (Key :type "Key Structure"))
  (:`Pressed`
    (bind _result (`/Engine/EditorBlueprintResources/StandardMacros.IncrementInt` (`self.Seed`))
      (:`  `
        (set `self.Seed` (`KismetMathLibrary.Clamp` _result 1 4))))))

(event `Key|MouseScrollDown`
  (params (Key :type "Key Structure"))
  (:`Pressed`
    (bind _result (`/Engine/EditorBlueprintResources/StandardMacros.DecrementInt` (`self.Seed`))
      (:`  `
        (set `self.Seed` (`KismetMathLibrary.Clamp` _result 1 4))))))

(fn `UserConstructionScript`)