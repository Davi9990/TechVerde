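; Blueprint for a purchasable area unlock, where the player pays money to remove fences blocking an area.
; TentarDesbloquear compares the money manager's balance against the unlock price and spends it when sufficient.
; On success it destroys both fence components, the interaction collider and the 3D text.
; Otherwise it prints a Portuguese message saying there is not enough money.
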(event `TentarDesbloquear`
  (if (>= (`/Game/BluePrints/Dinheiro_Estações/BP_MoneyManager.Money` (`self.MoneyManagerRef`)) (`self.PrecoDesbloqueio`))
    (`/Game/BluePrints/Dinheiro_Estações/BP_MoneyManager.SpendMoney` (`self.MoneyManagerRef`) (`self.PrecoDesbloqueio`))
    (bind _output_get (set `self.CercasParaDeletar` (`|MakeArray` (`self.Cerca 2`) (`self.Cerca 1`))))
    (for _array_element _output_get
      (`ActorComponent.K2_DestroyComponent` _array_element))
    (`ActorComponent.K2_DestroyComponent` (`self.ColisorInteracao`))
    (`ActorComponent.K2_DestroyComponent` (`self.Text3D`))
    (else
      (`KismetSystemLibrary.PrintString` "voce nao tem dinheiro para desbloquear essa area"))))

(fn `UserConstructionScript`)