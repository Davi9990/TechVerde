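; Purchasable turbine that generates money for the player and can be upgraded, using the BP_MoneyManager found at BeginPlay.
; ComprarTurbina spends money to start the looping animation and a non-looping 30-second payout timer, then doubles the price shown on Text3D.
; A later purchase at level 2 raises the payout and removes the Box and price text.
; Scaling and level 3 logic are left unconnected.
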(event `ComprarTurbina`
  (if (`self.Comprada?`)
    (if (>= (`/Game/BluePrints/Dinheiro_Estações/BP_MoneyManager.Money` (`self.MoneyRef`)) (`self.PrecoAquisicao`))
      (`/Game/BluePrints/Dinheiro_Estações/BP_MoneyManager.SpendMoney` (`self.MoneyRef`) (`self.PrecoAquisicao`))
      (switch `int` (`self.NivelAtual`)
        (:`2`
          (set `self.DinheiroGerado` 75000)
          (set `self.PrecoAquisicao` 500000)
          (bind _result (`/Engine/EditorBlueprintResources/StandardMacros.IncrementInt` (`self.NivelAtual`))
            (:`  `
              (set `self.NivelAtual` _result)
              (`ActorComponent.K2_DestroyComponent` (`self.Box`))
              (`ActorComponent.K2_DestroyComponent` (`self.Text3D`))
              (`KismetSystemLibrary.PrintString` "Turbina nivel 2")))))
      (else
        (`KismetSystemLibrary.PrintString` "Sem dinheiro para subir de nivel")))
    (elif (>= (`/Game/BluePrints/Dinheiro_Estações/BP_MoneyManager.Money` (`self.MoneyRef`)) (`self.PrecoAquisicao`))
      (`/Game/BluePrints/Dinheiro_Estações/BP_MoneyManager.SpendMoney` (`self.MoneyRef`) (`self.PrecoAquisicao`))
      (set `self.Comprada?` true)
      (`SkeletalMeshComponent.PlayAnimation` (`self.Turbina_Animada`) "/Game/BluePrints/Turbina/Turbina_Animada_Anim.Turbina_Animada_Anim" true)
      (`KismetSystemLibrary.K2_SetTimerDelegate` (delegate `GerarRendimentoRoda`) 30.0)
      (set `self.PrecoAquisicao` (* (`self.PrecoAquisicao`) 2))
      (bind _result_2 (`/Engine/EditorBlueprintResources/StandardMacros.IncrementInt` (`self.NivelAtual`))
        (:`  `
          (set `self.NivelAtual` _result_2)
          (set `Text3DComponent.Text` (`|FormatText` "$ {Preco}" (`self.PrecoAquisicao`)) (`self.Text3D`))
          (`KismetSystemLibrary.PrintString` "Turbina ligou")))
      (else
        (`KismetSystemLibrary.PrintString` "sem dinheiro para comprar a roda")))))

(event `GerarRendimentoRoda`
  (`/Game/BluePrints/Dinheiro_Estações/BP_MoneyManager.AddMoney` (`self.MoneyRef`) (`self.DinheiroGerado`))
  (`KismetSystemLibrary.PrintString` "Turbina gerou dinheiro"))

(event `self.ReceiveBeginPlay`
  (bind _outactors (`GameplayStatics.GetAllActorsOfClass` "/Game/BluePrints/Dinheiro_Estações/BP_MoneyManager.BP_MoneyManager_C"))
  (set `self.MoneyRef` (`|GetArrayItem` _outactors))
  (set `Text3DComponent.Text` (`|FormatText` "$ {valorRoda}" (`self.PrecoAquisicao`)) (`self.Text3D`)))

(fn `UserConstructionScript`)