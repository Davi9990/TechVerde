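; Collectible item Blueprint that adds itself and its image to the Inventario_UI inventory when E is pressed, or plays a sound if Bloqueado.
; BP_Fznd overlapping the mesh shows prompt text rotated toward the player camera and enables input.
; Ativar disables box and mesh collision but leaves the actor visible, and end overlap also shows the text and enables input rather than reversing them.
; UsarItem is an empty event.
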(event `UsarItem`)

(event `Ativar`
  (bind _foundwidgets (`WidgetBlueprintLibrary.GetAllWidgetsOfClass` "/Game/BluePrints/Inventario/Inventario_UI.Inventario_UI_C"))
  (`/Game/BluePrints/Inventario/Inventario_UI.AdicionarItem` (`|GetArrayItem` _foundwidgets) (`self.ItemImagem`) self)
  (`self.SetActorHiddenInGame` false)
  (`PrimitiveComponent.SetCollisionEnabled` (`self.Box`) "NoCollision")
  (`PrimitiveComponent.SetCollisionEnabled` (`self.StaticMesh`) "NoCollision"))

(event `Key|E`
  (params (Key :type "Key Structure"))
  (:`Pressed`
    (if (`self.Bloqueado?`)
      (`GameplayStatics.PlaySound2D` null 1.0 1.0 0.0 null null)
      (else
        (`self.Ativar`)))))

(event `self.StaticMesh.OnComponentBeginOverlap`
  (params (OverlappedComponent :type "PrimitiveComponent Object Reference") (OtherActor :type "Actor Object Reference") (OtherComp :type "PrimitiveComponent Object Reference") (OtherBodyIndex :type Integer) (bFromSweep :type Boolean) (SweepResult :type "HitResult Structure (by ref)"))
  (bind _asbp_fznd (cast `/Game/BluePrints/Fznd/BP_Fznd` OtherActor))
  (`SceneComponent.SetHiddenInGame` (`self.TextRender`) false false)
  (`self.EnableInput` (`GameplayStatics.GetPlayerController` 0))
  (`SceneComponent.K2_SetWorldRotation` (`self.TextRender`) (`KismetMathLibrary.FindLookAtRotation` (`SceneComponent.K2_GetComponentLocation` (`self.TextRender`)) (`SceneComponent.K2_GetComponentLocation` (`/Game/BluePrints/Fznd/BP_Fznd.Camera` _asbp_fznd))) false false))

(event `self.StaticMesh.OnComponentEndOverlap`
  (params (OverlappedComponent :type "PrimitiveComponent Object Reference") (OtherActor :type "Actor Object Reference") (OtherComp :type "PrimitiveComponent Object Reference") (OtherBodyIndex :type Integer))
  (cast `/Game/BluePrints/Fznd/BP_Fznd` OtherActor)
  (`SceneComponent.SetHiddenInGame` (`self.TextRender`) false false)
  (`self.EnableInput` (`GameplayStatics.GetPlayerController` 0)))

(fn `UserConstructionScript`)