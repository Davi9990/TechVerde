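; AppleTree_BP is an apple tree that grows and bears fruit when its OnIrrigate event fires.
; The PlantGrow timeline reveals and scales up the Plants component, then on finishing starts a second timeline that reveals and scales up four apples.
; A Delay started from that second timeline's Update later swaps the apples' material to Food_paint_Mat.
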(event `self.ReceiveBeginPlay`)

(event `/Game/BluePrints/Plants/BP_Plants.On Irrigate`
  (bind _apple (`self.Apple`))
  (`SceneComponent.SetHiddenInGame` (`self.Plants`) false false)
  (bind (_direction _time_for_plants_grow) (`Timeline|Plant Grow` :!via `PlayFromStart`)
    (:`Update`
      (bind _returnvalue (`KismetMathLibrary.Lerp` 0.1 4.0 _time_for_plants_grow))
      (`SceneComponent.SetRelativeScale3D` (`self.Plants`) (`KismetMathLibrary.MakeVector` _returnvalue _returnvalue _returnvalue)))
    (:`Finished`
      (bind (_direction_2 _time_for_plants_grow_2) (`Timeline|Timeline` :!via `PlayFromStart`)
        (:`Update`
          (`SceneComponent.SetHiddenInGame` _apple false false)
          (`SceneComponent.SetHiddenInGame` (`self.Apple2`) false false)
          (`SceneComponent.SetHiddenInGame` (`self.Apple4`) false false)
          (`SceneComponent.SetHiddenInGame` (`self.Apple3`) false false)
          (bind _returnvalue_2 (`KismetMathLibrary.Lerp` 0.1 0.8 _time_for_plants_grow_2))
          (`SceneComponent.SetRelativeScale3D` _apple (`KismetMathLibrary.MakeVector` _returnvalue_2 _returnvalue_2 _returnvalue_2))
          (`SceneComponent.SetRelativeScale3D` (`self.Apple2`) (`KismetMathLibrary.MakeVector` _returnvalue_2 _returnvalue_2 _returnvalue_2))
          (`SceneComponent.SetRelativeScale3D` (`self.Apple3`) (`KismetMathLibrary.MakeVector` _returnvalue_2 _returnvalue_2 _returnvalue_2))
          (`SceneComponent.SetRelativeScale3D` (`self.Apple4`) (`KismetMathLibrary.MakeVector` _returnvalue_2 _returnvalue_2 _returnvalue_2))
          (`KismetSystemLibrary.Delay` 12.5)
          (`PrimitiveComponent.SetMaterial` (`self.Apple`) 0 "/Game/Assets/Cenario_Assets/Plantas/food_paint_Mat.food_paint_Mat")
          (`PrimitiveComponent.SetMaterial` (`self.Apple2`) 0 "/Game/Assets/Cenario_Assets/Plantas/food_paint_Mat.food_paint_Mat")
          (`PrimitiveComponent.SetMaterial` (`self.Apple3`) 0 "/Game/Assets/Cenario_Assets/Plantas/food_paint_Mat.food_paint_Mat")
          (`PrimitiveComponent.SetMaterial` (`self.Apple4`) 0 "/Game/Assets/Cenario_Assets/Plantas/food_paint_Mat.food_paint_Mat"))))))

(fn `UserConstructionScript`)