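; Farm tile that plants, grows and harvests wheat, carrot, corn or tomato.
; PlantSeed spends the player pawn's selected seed, then swaps meshes through timed stages with a Text3D countdown.
; A small random disease roll halts growth and applies a disabled material; the output named Disease is actually the healthy path.
; Activate harvests a FullyGrow tile, spawning any recorded crop's actor and clearing the tile for replanting.
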(event `self.ReceiveBeginPlay`
  (set `Text3DComponent.Text` (`self.Value`) (`self.Text3D`)))

(event `Plant Carrot`
  (bind _relativetransformlocation (`self.RelativeTransformLocation`))
  (bind _returnvalue (`AddComponent|NODE_AddStaticMeshComponent-9` :`RelativeTransform` (`KismetMathLibrary.MakeTransform` _relativetransformlocation)))
  (`self.GrowTime` (`self.CarrotTime`)
    (:`Out`
      (`self.ChanceOfDisease` _returnvalue
        (:`Disease`
          (`ActorComponent.K2_DestroyComponent` _returnvalue)
          (bind _returnvalue_2 (`AddComponent|NODE_AddStaticMeshComponent-10` :`RelativeTransform` (`KismetMathLibrary.MakeTransform` _relativetransformlocation)))
          (`self.GrowTime` (`self.CarrotTime`)
            (:`Out`
              (`ActorComponent.K2_DestroyComponent` _returnvalue_2)
              (bind _returnvalue_3 (`AddComponent|NODE_AddStaticMeshComponent-11` :`RelativeTransform` (`KismetMathLibrary.MakeTransform` _relativetransformlocation)))
              (set `self.FullyGrow?` true)
              (set `self.CurrentMash` _returnvalue_3)
              (set `self.WhatCanBeHarvested?` "Carrot"))))))))

(event `Plant Tomato`
  (bind _relativetransformlocation (`self.RelativeTransformLocation`))
  (bind _returnvalue (`AddComponent|NODE_AddStaticMeshComponent-6` :`RelativeTransform` (`KismetMathLibrary.MakeTransform` _relativetransformlocation)))
  (`self.GrowTime` (`self.TomatoTime`)
    (:`Out`
      (`self.ChanceOfDisease` _returnvalue
        (:`Disease`
          (`ActorComponent.K2_DestroyComponent` _returnvalue)
          (bind _returnvalue_2 (`AddComponent|NODE_AddStaticMeshComponent-7` :`RelativeTransform` (`KismetMathLibrary.MakeTransform` _relativetransformlocation)))
          (`self.GrowTime` (`self.TomatoTime`)
            (:`Out`
              (`ActorComponent.K2_DestroyComponent` _returnvalue_2)
              (bind _returnvalue_3 (`AddComponent|NODE_AddStaticMeshComponent-8` :`RelativeTransform` (`KismetMathLibrary.MakeTransform` _relativetransformlocation)))
              (set `self.FullyGrow?` true)
              (set `self.CurrentMash` _returnvalue_3)
              (set `self.WhatCanBeHarvested?` "Tomato"))))))))

(event `Plant Corn`
  (bind _relativetransformlocation (`self.RelativeTransformLocation`))
  (bind _returnvalue (`AddComponent|NODE_AddStaticMeshComponent-3` :`RelativeTransform` (`KismetMathLibrary.MakeTransform` _relativetransformlocation)))
  (`self.GrowTime` (`self.CornTime`)
    (:`Out`
      (`self.ChanceOfDisease` _returnvalue
        (:`Disease`
          (`ActorComponent.K2_DestroyComponent` _returnvalue)
          (bind _returnvalue_2 (`AddComponent|NODE_AddStaticMeshComponent-4` :`RelativeTransform` (`KismetMathLibrary.MakeTransform` _relativetransformlocation)))
          (`self.GrowTime` (`self.CornTime`)
            (:`Out`
              (`ActorComponent.K2_DestroyComponent` _returnvalue_2)
              (bind _returnvalue_3 (`AddComponent|NODE_AddStaticMeshComponent-5` :`RelativeTransform` (`KismetMathLibrary.MakeTransform` _relativetransformlocation)))
              (set `self.FullyGrow?` true)
              (set `self.CurrentMash` _returnvalue_3)
              (set `self.WhatCanBeHarvested?` "Corn"))))))))

(event `Plant Wheat`
  (bind _relativetransformlocation (`self.RelativeTransformLocation`))
  (bind _returnvalue (`AddComponent|NODE_AddStaticMeshComponent-0` :`RelativeTransform` (`KismetMathLibrary.MakeTransform` _relativetransformlocation)))
  (`self.GrowTime` (`self.WheelTime`)
    (:`Out`
      (`self.ChanceOfDisease` _returnvalue
        (:`Disease`
          (`ActorComponent.K2_DestroyComponent` _returnvalue)
          (bind _returnvalue_2 (`AddComponent|NODE_AddStaticMeshComponent-1` :`RelativeTransform` (`KismetMathLibrary.MakeTransform` _relativetransformlocation)))
          (`self.GrowTime` (`self.WheelTime`)
            (:`Out`
              (`ActorComponent.K2_DestroyComponent` _returnvalue_2)
              (bind _returnvalue_3 (`AddComponent|NODE_AddStaticMeshComponent-2` :`RelativeTransform` (`KismetMathLibrary.MakeTransform` _relativetransformlocation)))
              (`self.ChanceOfDisease` _returnvalue_3
                (:`Disease`
                  (set `self.FullyGrow?` true)
                  (set `self.CurrentMash` _returnvalue_3)
                  (set `self.WhatCanBeHarvested?` "Wheat"))))))))))

(event `/Game/BluePrints/Plants/Plantation/BPI_PlantSeed.PlantSeed`
  (`KismetSystemLibrary.PrintString` "Estou Passando!")
  (if (not (`self.IsSomentingPlanted?`))
    (bind _asbp_fznd (cast `/Game/BluePrints/Fznd/BP_Fznd` (`GameplayStatics.GetPlayerPawn` 0))
      (:`then`
        (switch `int` (`/Game/BluePrints/Fznd/BP_Fznd.Seed` _asbp_fznd)
          (:`1`
            (`self.DoWeHaveWheatSeed`
              (:`Output`
                (`self.Plant Wheat`))))
          (:`2`
            (`self.DoWeHaveCarrotSeed`
              (:`Output`
                (`self.Plant Carrot`))))
          (:`3`
            (`self.DoWeHaveCornSeed`
              (:`Output`
                (`self.Plant Corn`))))
          (:`4`
            (`self.DoWeHaveTomatoSeed`
              (:`Output`
                (`self.Plant Tomato`)))))
        (set `self.IsSomentingPlanted?` true))
      (:`CastFailed`
        (`KismetSystemLibrary.PrintString` "CastFalhou")))))

(event `/Game/BluePrints/Plants/Plantation/BPI_Activate.Activate`
  (`self.Harvest`))

(fn `Harvest`
  (bind _returnvalue (`KismetMathLibrary.Conv_VectorToTransform` (`SceneComponent.K2_GetComponentLocation` (`self.Text3D`))))
  (if (`self.FullyGrow?`)
    (`ActorComponent.K2_DestroyComponent` (`self.CurrentMash`))
    (switch `string` (`self.WhatCanBeHarvested?`)
      (:`Default`
        _)
      (:`Wheat`
        (`|SpawnActorFromClass` "/Game/BluePrints/Plants/Wheel/BP_WheatLoser.BP_WheatLoser_C" _returnvalue "Undefined" "MultiplyWithRoot" null null))
      (:`Carrot`
        (`|SpawnActorFromClass` "/Game/BluePrints/Plants/Carrot/BP_CarrotLoser.BP_CarrotLoser_C" _returnvalue "Undefined" "MultiplyWithRoot" null null))
      (:`Corn`
        (`|SpawnActorFromClass` "/Game/BluePrints/Plants/Corn/BP_CornLoser.BP_CornLoser_C" _returnvalue "Undefined" "MultiplyWithRoot" null null))
      (:`Tomato`
        (`|SpawnActorFromClass` "/Game/BluePrints/Plants/Tomato/BP_TomatoLoser.BP_TomatoLoser_C" _returnvalue "Undefined" "MultiplyWithRoot" null null)))
    (set `self.FullyGrow?` false)
    (set `self.CurrentMash` null)
    (set `self.IsSomentingPlanted?` false)
    (set `self.WhatCanBeHarvested?` "")))

(fn `UserConstructionScript`)