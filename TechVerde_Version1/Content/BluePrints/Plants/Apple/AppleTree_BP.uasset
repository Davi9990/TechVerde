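; Apple tree plant Blueprint that grows the tree and then its fruit when irrigated.
; The OnIrrigate event unhides the plant and scales it up with the PlantGrow timeline.
; When that finishes, a second timeline scales up the apple components, unhiding most of them.
; A delay started from that timeline's update later swaps the apples' material to a food paint material.
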(event `/Game/BluePrints/Plants/Apple/BP_Plants.On Irrigate`
  (bind _apple3 (`self.Apple3`))
  (`SceneComponent.SetHiddenInGame` (`self.Plants`) false false)
  (bind (_direction _time_for_plants_grow) (`Timeline|Plant Grow` :!via `PlayFromStart`)
    (:`Update`
      (bind _returnvalue (`KismetMathLibrary.Lerp` 0.1 2.8 _time_for_plants_grow))
      (`SceneComponent.SetRelativeScale3D` (`self.Plants`) (`KismetMathLibrary.MakeVector` _returnvalue _returnvalue _returnvalue)))
    (:`Finished`
      (bind (_direction_2 _time_for_plants_grow_2) (`Timeline|Timeline` :!via `PlayFromStart`)
        (:`Update`
          (`SceneComponent.SetHiddenInGame` _apple3 false false)
          (`SceneComponent.SetHiddenInGame` (`self.Apple0`) false false)
          (`SceneComponent.SetHiddenInGame` (`self.Apple1`) false false)
          (`SceneComponent.SetHiddenInGame` (`self.Apple4`) false false)
          (`SceneComponent.SetHiddenInGame` (`self.Apple5`) false false)
          (`SceneComponent.SetHiddenInGame` (`self.Apple6`) false false)
          (`SceneComponent.SetHiddenInGame` (`self.Apple7`) false false)
          (`SceneComponent.SetHiddenInGame` (`self.Apple8`) false false)
          (`SceneComponent.SetHiddenInGame` (`self.Apple9`) false false)
          (`SceneComponent.SetHiddenInGame` (`self.Apple11`) false false)
          (`SceneComponent.SetHiddenInGame` (`self.Apple12`) false false)
          (bind _returnvalue_2 (`KismetMathLibrary.Lerp` 0.01 0.2 _time_for_plants_grow_2))
          (`SceneComponent.SetRelativeScale3D` _apple3 (`KismetMathLibrary.MakeVector` _returnvalue_2 _returnvalue_2 _returnvalue_2))
          (`SceneComponent.SetRelativeScale3D` (`self.Apple0`) (`KismetMathLibrary.MakeVector` _returnvalue_2 _returnvalue_2 _returnvalue_2))
          (`SceneComponent.SetRelativeScale3D` (`self.Apple1`) (`KismetMathLibrary.MakeVector` _returnvalue_2 _returnvalue_2 _returnvalue_2))
          (`SceneComponent.SetRelativeScale3D` (`self.Apple2`) (`KismetMathLibrary.MakeVector` _returnvalue_2 _returnvalue_2 _returnvalue_2))
          (`SceneComponent.SetRelativeScale3D` (`self.Apple4`) (`KismetMathLibrary.MakeVector` _returnvalue_2 _returnvalue_2 _returnvalue_2))
          (`SceneComponent.SetRelativeScale3D` (`self.Apple5`) (`KismetMathLibrary.MakeVector` _returnvalue_2 _returnvalue_2 _returnvalue_2))
          (`SceneComponent.SetRelativeScale3D` (`self.Apple6`) (`KismetMathLibrary.MakeVector` _returnvalue_2 _returnvalue_2 _returnvalue_2))
          (`SceneComponent.SetRelativeScale3D` (`self.Apple7`) (`KismetMathLibrary.MakeVector` _returnvalue_2 _returnvalue_2 _returnvalue_2))
          (`SceneComponent.SetRelativeScale3D` (`self.Apple8`) (`KismetMathLibrary.MakeVector` _returnvalue_2 _returnvalue_2 _returnvalue_2))
          (`SceneComponent.SetRelativeScale3D` (`self.Apple10`) (`KismetMathLibrary.MakeVector` _returnvalue_2 _returnvalue_2 _returnvalue_2))
          (`SceneComponent.SetRelativeScale3D` (`self.Apple9`) (`KismetMathLibrary.MakeVector` _returnvalue_2 _returnvalue_2 _returnvalue_2))
          (`SceneComponent.SetRelativeScale3D` (`self.Apple11`) (`KismetMathLibrary.MakeVector` _returnvalue_2 _returnvalue_2 _returnvalue_2))
          (`SceneComponent.SetRelativeScale3D` (`self.Apple12`) (`KismetMathLibrary.MakeVector` _returnvalue_2 _returnvalue_2 _returnvalue_2))
          (`KismetSystemLibrary.Delay` 10.0)
          (`PrimitiveComponent.SetMaterial` (`self.Apple3`) 0 "/Game/Assets/Cenario_Assets/Plantas/food_paint_Mat.food_paint_Mat")
          (`PrimitiveComponent.SetMaterial` (`self.Apple0`) 0 "/Game/Assets/Cenario_Assets/Plantas/food_paint_Mat.food_paint_Mat")
          (`PrimitiveComponent.SetMaterial` (`self.Apple6`) 0 "/Game/Assets/Cenario_Assets/Plantas/food_paint_Mat.food_paint_Mat")
          (`PrimitiveComponent.SetMaterial` (`self.Apple5`) 0 "/Game/Assets/Cenario_Assets/Plantas/food_paint_Mat.food_paint_Mat")
          (`PrimitiveComponent.SetMaterial` (`self.Apple12`) 0 "/Game/Assets/Cenario_Assets/Plantas/food_paint_Mat.food_paint_Mat")
          (`PrimitiveComponent.SetMaterial` (`self.Apple11`) 0 "/Game/Assets/Cenario_Assets/Plantas/food_paint_Mat.food_paint_Mat")
          (`PrimitiveComponent.SetMaterial` (`self.Apple10`) 0 "/Game/Assets/Cenario_Assets/Plantas/food_paint_Mat.food_paint_Mat")
          (`PrimitiveComponent.SetMaterial` (`self.Apple9`) 0 "/Game/Assets/Cenario_Assets/Plantas/food_paint_Mat.food_paint_Mat")
          (`PrimitiveComponent.SetMaterial` (`self.Apple8`) 0 "/Game/Assets/Cenario_Assets/Plantas/food_paint_Mat.food_paint_Mat")
          (`PrimitiveComponent.SetMaterial` (`self.Apple7`) 0 "/Game/Assets/Cenario_Assets/Plantas/food_paint_Mat.food_paint_Mat")
          (`PrimitiveComponent.SetMaterial` (`self.Apple4`) 0 "/Game/Assets/Cenario_Assets/Plantas/food_paint_Mat.food_paint_Mat")
          (`PrimitiveComponent.SetMaterial` (`self.Apple2`) 0 "/Game/Assets/Cenario_Assets/Plantas/food_paint_Mat.food_paint_Mat")
          (`PrimitiveComponent.SetMaterial` (`self.Apple1`) 0 "/Game/Assets/Cenario_Assets/Plantas/food_paint_Mat.food_paint_Mat"))))))

(fn `UserConstructionScript`)