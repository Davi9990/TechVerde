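; BP_CarrotLoser is a carrot plant pickup that counts toward the overlapping BP_Fznd actor's carrot tally and pays out money.
; On BeginPlay it caches the first BP_MoneyManager found in the level.
; When a BP_Fznd enters its Box, it increments that actor's AmountOfCarrot, destroys itself and calls AddMoney on the manager with ValorPlantaCarrot.
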(event `self.ReceiveBeginPlay`
  (bind _outactors (`GameplayStatics.GetAllActorsOfClass` "/Game/BluePrints/Dinheiro_Estações/BP_MoneyManager.BP_MoneyManager_C"))
  (set `self.Money Ref Carrot` (`|GetArrayItem` _outactors)))

(event `self.Box.OnComponentBeginOverlap`
  (params (OverlappedComponent :type "PrimitiveComponent Object Reference") (OtherActor :type "Actor Object Reference") (OtherComp :type "PrimitiveComponent Object Reference") (OtherBodyIndex :type Integer) (bFromSweep :type Boolean) (SweepResult :type "HitResult Structure (by ref)"))
  (bind _asbp_fznd (cast `/Game/BluePrints/Fznd/BP_Fznd` OtherActor))
  (bind _result (`/Engine/EditorBlueprintResources/StandardMacros.IncrementInt` (`/Game/BluePrints/Fznd/BP_Fznd.AmountOfCarrot` _asbp_fznd))
    (:`  `
      (set `/Game/BluePrints/Fznd/BP_Fznd.AmountOfCarrot` _result _asbp_fznd)
      (`self.K2_DestroyActor`)
      (`/Game/BluePrints/Dinheiro_Estações/BP_MoneyManager.AddMoney` (`self.Money Ref Carrot`) (`self.Valor Planta Carrot`)))))

(fn `UserConstructionScript`)