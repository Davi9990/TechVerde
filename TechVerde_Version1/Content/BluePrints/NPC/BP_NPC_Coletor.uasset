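; BP_NPC_Coletor is an NPC that collects stored money from a target station and returns to its starting spot.
; On BeginPlay it saves its home transform and starts a looping timer that checks whether the station's StoredMoney has reached its maximum.
; When full, it AI-moves to the station's purchase collider, calls ColetarDinheiro, faces the station, waits, then walks home and restores its original rotation.
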(event `self.ReceiveBeginPlay`
  (set `self.HomeLocation` (`self.K2_GetActorLocation`))
  (set `self.HomeRotation` (`self.K2_GetActorRotation`))
  (`KismetSystemLibrary.K2_SetTimerDelegate` (delegate `VerificarEstacao`) 10.0 true))

(event `VerificarEstacao`
  (bind _targetstationreference (`self.TargetStationReference`))
  (bind _targetstationreference_2 (`self.TargetStationReference`))
  (if (>= (`/Game/BluePrints/Dinheiro_Estações/BP_AnimalStation.StoredMoney` _targetstationreference) (`/Game/BluePrints/Dinheiro_Estações/BP_AnimalStation.MaxStoredMoney` _targetstationreference))
    (`|AIMoveTo` self (`SceneComponent.K2_GetComponentLocation` (`/Game/BluePrints/Dinheiro_Estações/BP_AnimalStation.ColisorCompra` _targetstationreference_2)) null 1.0
      (:`OnSuccess`
        (`/Game/BluePrints/Dinheiro_Estações/BP_AnimalStation.ColetarDinheiro` _targetstationreference_2)
        (`self.K2_SetActorRotation` self (`KismetMathLibrary.FindLookAtRotation` (`self.K2_GetActorLocation`) (`SceneComponent.K2_GetComponentLocation` (`/Game/BluePrints/Dinheiro_Estações/BP_AnimalStation.DefaultSceneRoot` _targetstationreference_2))) false)
        (`KismetSystemLibrary.Delay` 5.0)
        (`|AIMoveTo` self (`self.HomeLocation`) null 1.0
          (:`OnSuccess`
            (`self.K2_SetActorRotation` (`self.HomeRotation`))))))))

(fn `UserConstructionScript`)