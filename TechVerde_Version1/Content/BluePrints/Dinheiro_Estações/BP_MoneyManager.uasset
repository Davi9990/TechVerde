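; BP_MoneyManager is an actor that tracks a Money balance, reset to zero on BeginPlay.
; AddMoney increases the balance, while SpendMoney deducts only when funds suffice, otherwise printing "Dinheiro Insuficiente" (insufficient money).
; Number keys 1–3 act as debug triggers for adding, spending and querying, each printing the balance.
; GetMoney returns without an explicit value, and the overlap event is empty.
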(event `self.ReceiveBeginPlay`
  (set `self.Money` 0))

(event `Key|One`
  (params (Key :type "Key Structure"))
  (:`Pressed`
    (`self.AddMoney` 50)
    (`KismetSystemLibrary.PrintString` (`KismetStringLibrary.Conv_IntToString` (`self.Money`)))))

(event `Key|Two`
  (params (Key :type "Key Structure"))
  (:`Pressed`
    (`self.SpendMoney` 20)
    (`KismetSystemLibrary.PrintString` (`KismetStringLibrary.Conv_IntToString` (`self.Money`)))))

(event `self.ReceiveActorBeginOverlap`
  (params (OtherActor :type "Actor Object Reference")))

(event `Key|Three`
  (params (Key :type "Key Structure"))
  (:`Pressed`
    (`self.GetMoney`)
    (`KismetSystemLibrary.PrintString` (`KismetStringLibrary.Conv_IntToString` (`self.Money`)))))

(fn `AddMoney`
  (params (Amount :type Integer :default 100))
  (set `self.Money` (+ (`self.Money`) Amount))
  (return))

(fn `GetMoney`
  (return))

(fn `SpendMoney`
  (params (Amount :type Integer))
  (returns (Success :type Boolean))
  (if (>= (`self.Money`) Amount)
    (set `self.Money` (- (`self.Money`) Amount))
    (return true)
    (else
      (`KismetSystemLibrary.PrintString` "Dinheiro Insuficiente"))))

(fn `UserConstructionScript`)