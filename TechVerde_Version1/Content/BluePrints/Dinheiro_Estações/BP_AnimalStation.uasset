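; BP_AnimalStation is a money station actor that sells animals for a pen and holds stored money.
; Interagir buys an animal when IsUnlocked, spawning it at one of five spawn points via BP_MoneyManager funds; otherwise it pays StoredMoney into the manager.
; GenerateIncome adds capped per-animal income, but its looping timer setup is disconnected, so nothing in this file triggers it.
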(event `self.ReceiveBeginPlay`
  (set `self.ListaDeSpawns` (`|MakeArray` (`self.SpawnPoint`) (`self.SpawnPoint2`) (`self.SpawnPoint3`) (`self.SpawnPoint4`) (`self.SpawnPoint1`)))
  (bind _outactors (`GameplayStatics.GetAllActorsOfClass` "/Game/BluePrints/Dinheiro_Estações/BP_MoneyManager.BP_MoneyManager_C"))
  (set `self.MoneyManagerReference` (`|GetArrayItem` _outactors)))

(event `Interagir`
  (if (`self.IsUnlocked`)
    (`self.TryPurchaseAnimal`)
    (else
      (`/Game/BluePrints/Dinheiro_Estações/BP_MoneyManager.AddMoney` (`self.MoneyManagerReference`) (`self.StoredMoney`))
      (set `self.StoredMoney` 0))))

(event `IncomeTimer`)

(fn `GenerateIncome`
  (set `self.StoredMoney` (`KismetMathLibrary.Clamp` (+ (* (`self.AnimalCount`) (`self.MoneyPerAnimal`)) (`self.StoredMoney`)) 0 (`self.MaxStoredMoney`))))

(fn `TryPurchaseAnimal`
  (if (< (`self.AnimalCount`) 5)
    (bind _output_get (set `self.MoneyManagerReference` (`self.MoneyManagerReference`)))
    (if (>= (`/Game/BluePrints/Dinheiro_Estações/BP_MoneyManager.Money` _output_get) (`self.AnimalPrice`))
      (`/Game/BluePrints/Dinheiro_Estações/BP_MoneyManager.SpendMoney` _output_get (`self.AnimalPrice`))
      (`|SpawnActorFromClass` (`self.AnimalClass`) (`SceneComponent.K2_GetComponentToWorld` (`|GetArrayItem` (`self.ListaDeSpawns`) (`self.AnimalCount`))) "Undefined" "MultiplyWithRoot" null null)
      (set `self.AnimalCount` (+ (`self.AnimalCount`) 1)))
    (else
      (`KismetSystemLibrary.PrintString` "Curral cheio"))))

(fn `UserConstructionScript`)