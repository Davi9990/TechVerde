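; Camera is a pawn Blueprint that drives movement and facing for what appears to be the protagonist.
; The forward/back axis adds movement on world X and Y together, producing diagonal travel independent of view or actor facing.
; When the input is non-zero, RInterpTo smoothly turns the actor toward that diagonal.
; The left/right axis event and construction script are empty, and the graph contains no camera logic.
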(event `InputAxis|Prota_Frente_e_tras`
  (params (AxisValue :type "Float (single-precision)"))
  (`self.AddMovementInput` (1.0 0.0 0.0) AxisValue)
  (`self.AddMovementInput` (0.0 1.0 0.0) (stale `InputAxis|Prota_esquerda_e_direita` AxisValue))
  (bind _returnvalue (`KismetMathLibrary.MakeVector` AxisValue (stale `InputAxis|Prota_esquerda_e_direita` AxisValue)))
  (if (> (`KismetMathLibrary.VSize` _returnvalue) 0.0)
    (`self.K2_SetActorRotation` (`KismetMathLibrary.RInterpTo` (`self.K2_GetActorRotation`) (`KismetMathLibrary.Conv_VectorToRotator` _returnvalue) (`GameplayStatics.GetWorldDeltaSeconds`) 10.0))))

(event `InputAxis|Prota_esquerda_e_direita`
  (params (AxisValue :type "Float (single-precision)")))

(fn `UserConstructionScript`)